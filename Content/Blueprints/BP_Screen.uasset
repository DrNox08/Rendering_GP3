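; BP_Screen is an actor with a plane that cycles through three texture choices when the player presses T.
; On BeginPlay it creates a dynamic material instance from the plane's first material and enables input from player controller 0.
; Each T press advances a wrapping index and writes it to the TextureIndex scalar parameter, so the material decides which image shows.
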(event EventBeginPlay
  (bind _plane (Variables|Default|GetPlane))
  (bind _returnvalue (Rendering|Material|CreateDynamicMaterialInstance _plane 0 (Rendering|Material|GetMaterial _plane 0) "None" :!class /Script/Engine.PrimitiveComponent))
  (Variables|Default|SetMIDR _returnvalue)
  (Input|EnableInput (Game|GetPlayerController 0)))

(event Input|KeyboardEvents|T
  (params (Key :type Key%20Structure :default "None"))
  (:Pressed
    (bind _output_get (Variables|Default|SetCurrentIndex (Math|Integer|%(Integer) (+ (Variables|Default|GetCurrentIndex) 1) 3)))
    (Rendering|Material|SetScalarParameterValue (Variables|Default|GetMIDR) "TextureIndex" (Math|Conversions|ToFloat(Integer) _output_get) :!class /Script/Engine.MaterialInstanceDynamic)))

(fn ConstructionScript)