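; Trigger-box actor that pulses a light while a Character stands inside, driven by a Material Parameter Collection.
; Overlap begin writes a blink start time and active flag to MPC_PulsingLight; overlap end clears the flag.
; With UseLight valid, BeginPlay tints the PointLight from EmissiveColor, and Tick recomputes a clamped sine intensity from collection parameters read through the MPC variable.
; Otherwise the light is zeroed and the collection's Glow is raised.
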(event OnComponentBeginOverlap(Box)
  (params (OverlappedComponent :type Primitive%20Component%20Object%20Reference) (OtherActor :type Actor%20Object%20Reference) (OtherComp :type Primitive%20Component%20Object%20Reference) (OtherBodyIndex :type Integer) (bFromSweep :type Boolean) (SweepResult :type Hit%20Result%20Structure%20%28by%20ref%29))
  (Utilities|Casting|CastToCharacter OtherActor)
  (Rendering|Material|SetScalarParameterValue "/Game/Materials/Collections/MPC_PulsingLight.MPC_PulsingLight" "BlinkStartTime" (Utilities|Time|GetGameTimeinSeconds) :!class /Script/Engine.KismetMaterialLibrary)
  (Rendering|Material|SetScalarParameterValue "/Game/Materials/Collections/MPC_PulsingLight.MPC_PulsingLight" "BlinkActive" 1.0 :!class /Script/Engine.KismetMaterialLibrary))

(event OnComponentEndOverlap(Box)
  (params (OverlappedComponent :type Primitive%20Component%20Object%20Reference) (OtherActor :type Actor%20Object%20Reference) (OtherComp :type Primitive%20Component%20Object%20Reference) (OtherBodyIndex :type Integer))
  (Utilities|Casting|CastToCharacter OtherActor)
  (Rendering|Material|SetScalarParameterValue "/Game/Materials/Collections/MPC_PulsingLight.MPC_PulsingLight" "BlinkActive" 0.0 :!class /Script/Engine.KismetMaterialLibrary))

(event EventTick
  (params (DeltaSeconds :type Float%20%28single-precision%29))
  ;[0 0.003405 0.15 0.5] Serve solo per la luce
  (Variables|Components|GetUseLight
    (:then
      (CallFunction|GetMPCParams)
      (Rendering|Components|Light|SetIntensity (Variables|Default|GetPointLight) (CallFunction|GetLightValue)))
    (:else)))

(event EventBeginPlay
  (Variables|Components|GetUseLight
    (:then
      (bind _returnvalue (Rendering|Material|GetVectorParameterValue (Variables|MPC|GetMPC) (Utilities|Name|MakeLiteralName "EmissiveColor") :!class /Script/Engine.KismetMaterialLibrary))
      (Rendering|Components|Light|SetLightColor (Variables|Default|GetPointLight) _returnvalue true))
    (:else
      (Rendering|Components|Light|SetIntensity (Variables|Default|GetPointLight) 0.0)
      (Rendering|Material|SetScalarParameterValue "/Game/Materials/Collections/MPC_PulsingLight.MPC_PulsingLight" (Utilities|Name|MakeLiteralName "Glow") 2e+02 :!class /Script/Engine.KismetMaterialLibrary))))

(fn ConstructionScript)

(fn GetMPCParams
  (bind _returnvalue (Rendering|Material|GetScalarParameterValue (Variables|MPC|GetMPC) (Utilities|Name|MakeLiteralName "BlinkStartTime") :!class /Script/Engine.KismetMaterialLibrary))
  (Variables|Default|SetBlinkStartTime _returnvalue)
  (bind _returnvalue_2 (Rendering|Material|GetScalarParameterValue (Variables|MPC|GetMPC) (Utilities|Name|MakeLiteralName "BlinkSpeed") :!class /Script/Engine.KismetMaterialLibrary))
  (Variables|Default|SetBlinkSpeed _returnvalue_2)
  (bind _returnvalue_3 (Rendering|Material|GetScalarParameterValue (Variables|MPC|GetMPC) (Utilities|Name|MakeLiteralName "BlinkActive") :!class /Script/Engine.KismetMaterialLibrary))
  (Variables|Default|SetBlinkActive _returnvalue_3))

(fn GetLightValue
  (return (* (* (Math|Float|Max(Float) (Math|Trig|Sin(Radians) (* (* (- (Utilities|Time|GetGameTimeinSeconds) (Variables|Default|GetBlinkStartTime)) (Variables|Default|GetBlinkSpeed)) 6.2832)) 0.0) (Variables|Default|GetBlinkActive)) (Variables|Components|GetMaxLightIntensity))))